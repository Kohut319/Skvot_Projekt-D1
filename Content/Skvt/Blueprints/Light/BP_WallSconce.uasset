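; BP_WallSconce is a wall sconce light actor with an adjustable cone-shaped light that can be switched on and off.
; The construction script applies the on state, brightness, color and inner and outer cone angles to the SconceLight component from the actor's variables.
; ToggleON stores the passed state in ItsON and updates the light's visibility to match.
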(fn `ToggleON`
  (params (`Is On` :type Boolean))
  (bind _output_get (set `self.Its ON` `Is On`))
  (`SceneComponent.SetVisibility` (`self.SconceLight`) _output_get false))

(fn `UserConstructionScript`
  (bind _sconcelight (`self.SconceLight`))
  (`SceneComponent.SetVisibility` _sconcelight (`self.Its ON`) false)
  (`LightComponent.SetIntensity` _sconcelight (`self.Brightness`))
  (`LightComponent.SetLightColor` _sconcelight (`self.Color`) true)
  (`SpotLightComponent.SetInnerConeAngle` _sconcelight (`self.Inner Cone Angle`))
  (`SpotLightComponent.SetOuterConeAngle` _sconcelight (`self.Outer Cone Angle`)))